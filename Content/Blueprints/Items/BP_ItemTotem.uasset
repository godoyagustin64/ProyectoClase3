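; BP_ItemTotem is a totem item that rotates about its yaw axis, one time, when activated.
; On BeginPlay it caches the mesh's world rotation and clears its activated flag.
; ActivateTotemBP plays a stone-dragging sound and runs a Timeline that adds a yaw offset to the cached rotation, applied to the whole actor.
; The activated flag is set only when the Timeline finishes, blocking later activations from that point.
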(event `self.ReceiveBeginPlay`
  (set `self.RotacionInicial` (`SceneComponent.K2_GetComponentRotation` (`self.Mesh`)))
  (set `self.isActivated` false))

(event `self.ActivateTotemBP`
  (bind (_rotacioninicial_roll _rotacioninicial_pitch _rotacioninicial_yaw) (`KismetMathLibrary.BreakRotator` (`self.RotacionInicial`)))
  (if (not (`self.isActivated`))
    (`GameplayStatics.PlaySound2D` "/Game/Sounds/stone_dragging.stone_dragging" 1.0 1.0 0.0 null null)
    (bind (_direction _rotation) (`Timeline|Timeline` :`NewTime` 3.0)
      (:`Update`
        (`self.K2_SetActorRotation` (`KismetMathLibrary.MakeRotator` _rotacioninicial_roll _rotacioninicial_pitch (+ _rotacioninicial_yaw _rotation))))
      (:`Finished`
        (set `self.isActivated` true)))))

(fn `UserConstructionScript`)