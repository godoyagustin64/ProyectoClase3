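; BP_Puerta is a double-leaf sliding door that opens with a stone gate sound when OpenDoorBP is called.
; BeginPlay caches each leaf's relative location, and a Timeline adds its PuertaIzq and PuertaDer tracks to those X values to slide the leaves.
; The sound plays at the left leaf's cached relative location, passed as a world location.
; The file contains no closing logic or built-in trigger.
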(event `self.ReceiveBeginPlay`
  (set `self.PosicionIzqInicial` (`SceneComponent.RelativeLocation` (`self.HojaIzquierda`)))
  (set `self.PosicionDerInicial` (`SceneComponent.RelativeLocation` (`self.HojaDerecha`))))

(event `self.OpenDoorBP`
  (bind (_posicionizqinicial_x _posicionizqinicial_y _posicionizqinicial_z) (`KismetMathLibrary.BreakVector` (`self.PosicionIzqInicial`)))
  (bind (_posicionderinicial_x _posicionderinicial_y _posicionderinicial_z) (`KismetMathLibrary.BreakVector` (`self.PosicionDerInicial`)))
  (`GameplayStatics.PlaySoundAtLocation` "/Game/Sounds/BIG_stone_gate_opening_7sec.BIG_stone_gate_opening_7sec" (`self.PosicionIzqInicial`) (struct) 1.0 1.0 0.0 null null null null)
  (bind (_direction _puertaizq _puertader) (`Timeline|Timeline` :`NewTime` 5.0)
    (:`Update`
      (`SceneComponent.K2_SetRelativeLocation` (`self.HojaIzquierda`) (`KismetMathLibrary.MakeVector` (+ _puertaizq _posicionizqinicial_x) _posicionizqinicial_y _posicionizqinicial_z) false false)
      (`SceneComponent.K2_SetRelativeLocation` (`self.HojaDerecha`) (`KismetMathLibrary.MakeVector` (+ _puertader _posicionderinicial_x) _posicionderinicial_y _posicionderinicial_z) false false))))

(fn `UserConstructionScript`)